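; Lobby HUD that creates and displays the lobby widget, shows the mouse cursor and refreshes the player list.
; A looping timer retries until the first player controller's PlayerState casts to BP_LobbyPlayerState.
; It then binds to that state's UpdatePlayerData dispatcher, triggers an initial list update through the widget and clears the timer.
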(event EventBeginPlay
  (bind _returnvalue (UserInterface|CreateWidget "/Game/ShootingGame/Widget/Lobby/Lobby_Widget.Lobby_Widget_C"))
  (bind _output_get (Variables|Default|SetLobbyWidget _returnvalue))
  (UserInterface|Viewport|AddtoViewport _output_get 0)
  (Variables|/Script/Engine.PlayerController|SetbShowMouseCursor (Game|GetPlayerController 0) true)
  (Utilities|Time|SetTimerbyFunctionName 0 "InitPlayerState" 0.5 true))

(fn ConstructionScript)

(fn UpdatePlayerList
  (bind _lobbywidget (Variables|Default|GetLobbyWidget))
  (Utilities|IsValid _lobbywidget
    (:Is%20Valid
      (Default|UpdatePlayerList _lobbywidget))))

(fn InitPlayerState
  (bind _asbp_lobby_player_state (Utilities|Casting|CastToBP_LobbyPlayerState (Variables|/Script/Engine.Controller|GetPlayerState (Game|GetPlayerController 0))))
  (EventDispatchers|BindEventtoEventDispatcherUpdatePlayerData _asbp_lobby_player_state (EventDispatchers|CreateEvent :!event UpdatePlayerList))
  (CallFunction|UpdatePlayerList)
  (Utilities|Time|ClearTimerbyFunctionName 0 "InitPlayerState"))