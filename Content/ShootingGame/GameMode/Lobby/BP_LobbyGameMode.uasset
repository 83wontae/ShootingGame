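; Lobby game mode that sets up each joining player's data and notifies lobby player controllers when players arrive or leave.
; On new-player start, it builds lobby data from the player's name and stores it in BP_LobbyPlayerState.
; It then loops over network player indices, calling login events on each BP_LobbyPlayerController, with a matching loop for logout.
; Post-login, start and logout events print log-only debug strings.
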(event EventOnLogout
  (params (ExitingController :type Controller%20Object%20Reference))
  (Development|PrintString (Utilities|String|Append "[OnLogout]" (Utilities|GetDisplayName ExitingController)) false true "(R=0.000000,G=0.660000,B=1.000000,A=1.000000)" 6e+01)
  ;[1 1 1] 모든 플레이어에게 새로 접속한 플레이어 알림
  (for _index (range 0 (Class|AdvancedSessionsLibrary|GetNumberOfNetworkPlayers))
    (bind _asbp_lobby_player_controller (Utilities|Casting|CastToBP_LobbyPlayerController (Game|GetPlayerController _index)))
    (Default|OnOtherPlayerLogout _asbp_lobby_player_controller ExitingController)))

(event EventPostLogin
  (params (NewPlayer :type Player%20Controller%20Object%20Reference))
  (Development|PrintString (Utilities|String|Append "[OnPostLogin]" (Utilities|GetDisplayName NewPlayer)) false true "(R=0.000000,G=0.660000,B=1.000000,A=1.000000)" 6e+01))

(event EventHandleStartingNewPlayer
  (params (NewPlayer :type Player%20Controller%20Object%20Reference))
  (Development|PrintString (Utilities|String|Append "[Handle Starting New Player]" (Utilities|GetDisplayName NewPlayer)) false true "(R=0.000000,G=0.660000,B=1.000000,A=1.000000)" 6e+01)
  ;[1 1 1] 접속시 플레이어의 정보 설정
  (bind _asbp_lobby_player_state (Utilities|Casting|CastToBP_LobbyPlayerState (Variables|/Script/Engine.Controller|GetPlayerState NewPlayer)))
  (Default|SetPlayerData _asbp_lobby_player_state (CallFunction|MakeLobbyPlayerData NewPlayer))
  ;[1 1 1] 모든 플레이어에게 새로 접속한 플레이어 알림
  (for _index (range 0 (Class|AdvancedSessionsLibrary|GetNumberOfNetworkPlayers))
    (bind _asbp_lobby_player_controller (Utilities|Casting|CastToBP_LobbyPlayerController (Game|GetPlayerController _index)))
    (Default|OnNewPlayerLogin _asbp_lobby_player_controller NewPlayer)))

(fn ConstructionScript)

(fn MakeLobbyPlayerData
  (params (PlayerController :type Player%20Controller%20Object%20Reference))
  (bind _output_get (LocalVariables|SetPlayerData (Utilities|Struct|MakeSt_LobbyPlayerData (Class|AdvancedSessionsLibrary|GetPlayerName PlayerController))))
  (return _output_get))