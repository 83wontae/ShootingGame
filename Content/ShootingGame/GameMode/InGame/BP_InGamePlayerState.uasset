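; Player state for the in-game mode of the shooting game, holding the player's data and current HP as RepNotify variables.
; When PlayerData changes, its notify resets CurHP to the data's MaxHP and broadcasts an update dispatcher.
; CurHP changes broadcast their own dispatcher.
; SetPlayerData assigns the data, and DecHP subtracts damage, clamps at zero and returns the remaining HP.
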(fn ConstructionScript)

(fn OnRepPlayerData
  (Development|PrintString "OnPlayerData" false true "(R=0.000000,G=0.660000,B=1.000000,A=1.000000)" 6e+01)
  (Variables|Default|SetCurHP (.maxhp (Variables|Default|GetPlayerData)))
  (Default|CallEventDispatcherUpdatePlayerData (Variables|Default|GetPlayerData)))

(fn SetPlayerData
  (params (PlayerData :type St%20in%20Game%20Player%20Data%20Structure))
  (Variables|Default|SetPlayerData PlayerData))

(fn OnRepCurHP
  (Default|CallEventDispatcherUpdateCurHP (Variables|Default|GetCurHP)))

(fn DecHP
  (params (DecValue :type Float%20%28single-precision%29))
  (bind _output_get (Variables|Default|SetCurHP (- (Variables|Default|GetCurHP) DecValue)))
  (if (<= _output_get 0.0)
    (Variables|Default|SetCurHP 0.0)
    (return (Variables|Default|GetCurHP))
    (else
      (return (Variables|Default|GetCurHP)))))