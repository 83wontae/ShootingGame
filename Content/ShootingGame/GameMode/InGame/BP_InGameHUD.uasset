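; BP_InGameHUD is the in-game HUD for the shooting game, creating InGame_Widget and showing the player's name, HP, crosshair and pickup guide.
; A looping timer retries until the local controller's BP_InGamePlayerState exists, then binds its player-data and current-HP dispatchers, pushes the initial data and clears itself.
; Update and visibility functions forward values straight to the widget, with HP drawn from the cached PlayerState.
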(event EventBeginPlay
  (bind _returnvalue (UserInterface|CreateWidget "/Game/ShootingGame/Widget/InGame/InGame_Widget.InGame_Widget_C"))
  (bind _output_get (Variables|Default|SetInGameWidget _returnvalue))
  (UserInterface|Viewport|AddtoViewport _output_get 0)
  (Utilities|Time|SetTimerbyFunctionName 0 "InitPlayerState" 0.5 true))

(fn ConstructionScript)

(fn UpdatePlayerData
  (params (PlayerData :type St%20in%20Game%20Player%20Data%20Structure))
  (bind (_name _maxhp) (Utilities|Struct|BreakSt_InGamePlayerData PlayerData))
  (bind _ingamewidget (Variables|Default|GetInGameWidget))
  (Default|SetName _ingamewidget _name)
  (Default|SetHP _ingamewidget (Variables|/Game/ShootingGame/GameMode/InGame/BP_InGamePlayerState.BP_InGamePlayerState_C|GetCurHP (Variables|Default|GetPlayerState)) _maxhp))

(fn ShowGuidePickUp
  (params (InVisibility :type ESlateVisibility%20Enum :default "Visible"))
  (Default|ShowGuidePickUp (Variables|Default|GetInGameWidget) InVisibility))

(fn ShowCrosshair
  (params (InVisibility :type ESlateVisibility%20Enum :default "Visible"))
  (Default|ShowCrosshair (Variables|Default|GetInGameWidget) InVisibility))

(fn UpdatePlayerHP
  (params (CurHP :type Float%20%28single-precision%29))
  (Default|SetHP (Variables|Default|GetInGameWidget) CurHP (.maxhp (Variables|/Game/ShootingGame/GameMode/InGame/BP_InGamePlayerState.BP_InGamePlayerState_C|GetPlayerData (Variables|Default|GetPlayerState)))))

(fn InitPlayerState
  (bind _asbp_in_game_player_state (Utilities|Casting|CastToBP_InGamePlayerState (Variables|/Script/Engine.Controller|GetPlayerState (Game|GetPlayerController 0))))
  (bind _output_get (Variables|Default|SetPlayerState _asbp_in_game_player_state))
  (EventDispatchers|BindEventtoEventDispatcherUpdatePlayerData _output_get (EventDispatchers|CreateEvent :!event UpdatePlayerData))
  (EventDispatchers|BindEventtoEventDispatcherUpdateCurHP _output_get (EventDispatchers|CreateEvent :!event UpdatePlayerHP))
  (CallFunction|UpdatePlayerData (Variables|/Game/ShootingGame/GameMode/InGame/BP_InGamePlayerState.BP_InGamePlayerState_C|GetPlayerData _output_get))
  (Utilities|Time|ClearTimerbyFunctionName 0 "InitPlayerState"))