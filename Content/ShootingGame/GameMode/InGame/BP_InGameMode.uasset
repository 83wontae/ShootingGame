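; BP_InGameMode is the in-game GameMode for the shooting game, handling player setup and join/leave notifications.
; When a new player starts, it builds player data from their name and a default max HP and stores it in BP_InGamePlayerState.
; It then loops through player controllers to announce the join through BP_InGamePlayerController, and does the same for departures on logout.
; Login, start and logout events also write log messages.
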(event EventOnLogout
  (params (ExitingController :type Controller%20Object%20Reference))
  (|CallParentFunction ExitingController)
  (Development|PrintString (Utilities|String|Append "[OnLogout]" (Utilities|GetDisplayName ExitingController)) false true "(R=0.000000,G=0.660000,B=1.000000,A=1.000000)" 6e+01)
  ;[1 1 1] 모든 플레이어에게 새로 접속한 플레이어 알림
  (for _index (range 0 (Class|AdvancedSessionsLibrary|GetNumberOfNetworkPlayers))
    (bind _asbp_in_game_player_controller (Utilities|Casting|CastToBP_InGamePlayerController (Game|GetPlayerController _index)))
    (Default|OnOtherPlayerLogout _asbp_in_game_player_controller ExitingController)))

(event EventPostLogin
  (params (NewPlayer :type Player%20Controller%20Object%20Reference))
  (|CallParentFunction NewPlayer)
  (Development|PrintString (Utilities|String|Append "[OnPostLogin]" (Utilities|GetDisplayName NewPlayer)) false true "(R=0.000000,G=0.660000,B=1.000000,A=1.000000)" 6e+01))

(event EventHandleStartingNewPlayer
  (params (NewPlayer :type Player%20Controller%20Object%20Reference))
  (|CallParentFunction NewPlayer)
  (Development|PrintString (Utilities|String|Append "[Handle Starting New Player]" (Utilities|GetDisplayName NewPlayer)) false true "(R=0.000000,G=0.660000,B=1.000000,A=1.000000)" 6e+01)
  ;[1 1 1] 접속시 플레이어의 정보 설정
  (bind _asbp_in_game_player_state (Utilities|Casting|CastToBP_InGamePlayerState (Variables|/Script/Engine.Controller|GetPlayerState NewPlayer)))
  (Default|SetPlayerData _asbp_in_game_player_state (CallFunction|MakePlayerData NewPlayer))
  ;[1 1 1] 모든 플레이어에게 새로 접속한 플레이어 알림
  (for _index (range 0 (Class|AdvancedSessionsLibrary|GetNumberOfNetworkPlayers))
    (bind _asbp_in_game_player_controller (Utilities|Casting|CastToBP_InGamePlayerController (Game|GetPlayerController _index)))
    (Default|OnNewPlayerLogin _asbp_in_game_player_controller NewPlayer)))

(fn ConstructionScript)

(fn MakePlayerData
  (params (PlayerController :type Player%20Controller%20Object%20Reference))
  (return (Utilities|Struct|MakeSt_InGamePlayerData (Class|AdvancedSessionsLibrary|GetPlayerName PlayerController) 1e+02)))