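; Networked pickup rifle that shows a HUD prompt on overlap, attaches to the character's Weapon socket, and requests ownership through the local player controller.
; Trigger events run a looping fire timer locally and relay through Req/Res events, with each tick playing the shoot montage.
; OnShoot, triggered from outside this graph, plays effects; only the owning local player line-traces from the spring arm and requests damage on hit characters.
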(event Custom|ResPressTrigger
  ;[1 1 1] 방아쇠 입력 처리
  (Utilities|Time|SetTimerbyFunctionName 0 "UpdateShooting" (Variables|Default|GetFireSpeed) true))

(event Custom|ResReleasedTrigger
  ;[1 1 1] 방아쇠 입력 처리
  (Utilities|Time|ClearTimerbyFunctionName 0 "UpdateShooting"))

(event Custom|ReqPressTrigger
  ;[1 0 0] (Server) 방아쇠 입력
  (CallFunction|ResPressTrigger))

(event Custom|ReqApplyDamage
  (params (DamagedActor :type Actor%20Object%20Reference%20%28by%20ref%29) (BaseDamage :type Float%20%28single-precision%29) (EventInstigator :type Controller%20Object%20Reference%20%28by%20ref%29) (DamageCauser :type Actor%20Object%20Reference) (DamageTypeClass :type Damage%20Type%20Class%20Reference))
  (Game|Damage|ApplyDamage DamagedActor BaseDamage EventInstigator DamageCauser DamageTypeClass))

(event Custom|ReqReleasedTrigger
  ;[1 0 0] (Server) 방아쇠 입력
  (CallFunction|ResReleasedTrigger))

(event EventOnShoot
  ;[1 1 1] 총알 발사 사운드, 이펙트
  (Audio|SpawnSound2D (Variables|Default|GetShootSound) 1.0 1.0 0.0 0)
  (Effects|SpawnEmitteratLocation (Variables|Default|GetMuzzleEffect) (Transformation|GetSocketLocation (Variables|Default|GetStaticMesh) "Muzzle") "0, 0, 0" "0.100000,0.100000,0.100000")
  (if (== (Components|GetOwner) (Game|GetPlayerController 0))
    (CallFunction|OnHit)))

(event Collision|EventActorBeginOverlap
  (params (OtherActor :type Actor%20Object%20Reference))
  (Development|PrintString (Utilities|GetDisplayName OtherActor))
  (if (== OtherActor (Game|Player|GetPlayerPawn 0))
    (CallFunction|ShowPickUpGuideUI "Visible")))

(event EventPressTrigger
  ;[1 1 1] 방아쇠 입력 요청
  (Utilities|Time|SetTimerbyFunctionName 0 "UpdateShooting" (Variables|Default|GetFireSpeed) true)
  (CallFunction|ReqPressTrigger))

(event Collision|EventActorEndOverlap
  (params (OtherActor :type Actor%20Object%20Reference))
  (if (== OtherActor (Game|Player|GetPlayerPawn 0))
    (CallFunction|ShowPickUpGuideUI "Collapsed")))

(event EventReleasedTrigger
  ;[1 1 1] 방아쇠 입력 요청
  (Utilities|Time|ClearTimerbyFunctionName 0 "UpdateShooting")
  (CallFunction|ReqReleasedTrigger))

(fn ConstructionScript)

(fn AttachtoCharacter
  (params (OwnCharacter :type Character%20Object%20Reference))
  (bind _staticmesh (Variables|Default|GetStaticMesh))
  (bind _staticmesh_2 (Variables|Default|GetStaticMesh))
  (bind _output_get (Variables|Default|SetOwnCharacter OwnCharacter))
  (Physics|SetSimulatePhysics _staticmesh false)
  (Collision|SetCollisionEnabled _staticmesh "NoCollision")
  (bind _returnvalue (Transformation|AttachComponentToComponent _staticmesh (Variables|/Script/Engine.Character|GetMesh _output_get) "Weapon" "SnapToTarget" "SnapToTarget" "KeepRelative" false))
  (if _returnvalue
    ;[1 1 1] 장착 성공
    (CallFunction|ReqSetOwner)
    (if (== (Variables|Default|GetOwnCharacter) (Game|Player|GetPlayerPawn 0))
      (CallFunction|ShowCrosshair "Visible"))
    (return true)
    (else
      ;[1 1 1] 장착 실패
      (Physics|SetSimulatePhysics _staticmesh_2 true)
      (Collision|SetCollisionEnabled _staticmesh_2 "QueryAndPhysics")
      (Variables|Default|SetOwnCharacter 0)
      (return false))))

(fn ShowPickUpGuideUI
  (params (InVisibility :type ESlateVisibility%20Enum :default "Visible"))
  (bind _asbp_in_game_hud (Utilities|Casting|CastToBP_InGameHUD (HUD|GetHUD (Game|GetPlayerController 0))))
  (Default|ShowGuidePickUp _asbp_in_game_hud InVisibility))

(fn ShowCrosshair
  (params (InVisibility :type ESlateVisibility%20Enum :default "Visible"))
  (bind _asbp_in_game_hud (Utilities|Casting|CastToBP_InGameHUD (HUD|GetHUD (Game|GetPlayerController 0))))
  (Default|ShowCrosshair _asbp_in_game_hud InVisibility))

(fn UpdateShooting
  (Utilities|IsValid (Variables|Default|GetOwnCharacter)
    (:Is%20Valid
      (bind _asbp_character (Utilities|Casting|CastToBP_Character (Variables|Default|GetOwnCharacter)))
      (Animation|Montage|MontagePlay (Components|SkeletalMesh|GetAnimInstance (Variables|/Script/Engine.Character|GetMesh _asbp_character)) "/Game/RifleAnimsetPro/Animations/Rifle_ShootOnce_Montage.Rifle_ShootOnce_Montage" 1.0 "MontageLength" 0.0 true))
    (:Is%20Not%20Valid
      (Utilities|Time|ClearTimerbyFunctionName 0 "UpdateShooting"))))

(fn OnHit
  (bind _owncharacter (Variables|Default|GetOwnCharacter))
  (bind _asbp_character (Utilities|Casting|CastToBP_Character _owncharacter))
  (bind (_outhit _returnvalue) (Collision|LineTraceForObjects (Transformation|GetWorldLocation (Variables|/Game/ShootingGame/GameMode/InGame/BP_Character.BP_Character_C|GetSpringArm _asbp_character)) (+ (Transformation|GetWorldLocation (Variables|/Game/ShootingGame/GameMode/InGame/BP_Character.BP_Character_C|GetSpringArm _asbp_character)) (* (Math|Vector|GetForwardVector (Pawn|GetControlRotation _owncharacter :!class /Script/Engine.Pawn)) (Variables|Default|GetEffectiveRange))) (Utilities|Array|MakeArray "ObjectTypeQuery1" "ObjectTypeQuery2" "ObjectTypeQuery3" "ObjectTypeQuery4" "ObjectTypeQuery5" "ObjectTypeQuery6") true (Utilities|Array|MakeArray (Variables|Default|GetOwnCharacter)) "ForDuration"))
  (if _returnvalue
    (Effects|SpawnEmitteratLocation "/Game/StarterContent/Particles/P_Explosion.P_Explosion" (.ImpactPoint (Collision|BreakHitResult _outhit)))
    (bind _asbp_character_2 (Utilities|Casting|CastToBP_Character (.HitActor (Collision|BreakHitResult _outhit))))
    (CallFunction|ReqApplyDamage _asbp_character_2 1e+01 (Pawn|GetController (Variables|Default|GetOwnCharacter)))))

(fn ReqSetOwner
  (bind _owncharacter (Variables|Default|GetOwnCharacter))
  (Utilities|IsValid _owncharacter
    (:Is%20Valid
      (bind _asbp_in_game_player_controller (Utilities|Casting|CastToBP_InGamePlayerController (Pawn|GetController _owncharacter)))
      (if (== _asbp_in_game_player_controller (Game|GetPlayerController 0))
        (Default|ReqSetOwner _asbp_in_game_player_controller self)))))

(fn DoDetach
  (bind _staticmesh (Variables|Default|GetStaticMesh))
  (Physics|SetSimulatePhysics _staticmesh true)
  (Collision|SetCollisionEnabled _staticmesh "QueryAndPhysics")
  (Transformation|DetachFromComponent _staticmesh "KeepWorld" "KeepWorld" "KeepRelative" true)
  (return false))

(fn InputF
  (params (Character :type Character%20Object%20Reference))
  (bind _asbp_character (Utilities|Casting|CastToBP_Character Character))
  (bind _returnvalue (CallFunction|AttachtoCharacter _asbp_character))
  (return _returnvalue))